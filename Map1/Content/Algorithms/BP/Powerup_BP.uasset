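; Powerup pickup actor that hovers and spins in place until something overlaps it.
; Each tick, HoverPerFrame bobs it around its starting height with a sine-driven Lerp, phase-offset randomly per instance, and adds delta-time-scaled yaw.
; Any actor overlap sets BlockPickup, spawns the pickup particle at player 0's location, disables mesh collision and destroys the actor, with no gameplay effect applied here.
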(event `self.ReceiveBeginPlay`
  (set `self.RestTransform` (`self.GetTransform`))
  (set `self.RandFloat` (`KismetMathLibrary.RandomFloat`)))

(event `self.ReceiveActorBeginOverlap`
  (params (OtherActor :type "Actor Object Reference"))
  (bind _returnvalue_location (`KismetMathLibrary.BreakTransform` (`self.GetTransform` (`GameplayStatics.GetPlayerPawn` 0))))
  (set `self.BlockPickup` true)
  (`|SpawnActorFromClass` (`self.PickupParticle`) (`KismetMathLibrary.Conv_VectorToTransform` _returnvalue_location) "Undefined" "OverrideRootScale" null null)
  (`PrimitiveComponent.SetCollisionEnabled` (`self.StaticMeshComponent`) "NoCollision")
  (`self.K2_DestroyActor`))

(event `self.ReceiveTick`
  (params (DeltaSeconds :type "Float (single-precision)"))
  (`self.HoverPerFrame`))

(fn `HoverPerFrame`
  (bind _resttransform (`self.RestTransform`))
  (bind _transform_z_margin (`self.Transform Z Margin`))
  ;[1 1 1] Z-Axis Floating
  (bind _output_get (set `self.Iteration1` (+ (`self.Iteration1`) (* (`self.FloatSpeed`) (`GameplayStatics.GetWorldDeltaSeconds`)))))
  (`self.K2_SetActorTransform` (`KismetMathLibrary.MakeTransform` (`KismetMathLibrary.MakeVector` (.x (.location _resttransform)) (.y (.location _resttransform)) (`KismetMathLibrary.Lerp` (+ (.z (.location _resttransform)) _transform_z_margin) (+ (* (/ _transform_z_margin 2.0) -1.0) (.z (.location _resttransform))) (+ (* (`KismetMathLibrary.Sin` (+ _output_get (`self.RandFloat`))) 0.5) 0.5))) (`KismetMathLibrary.MakeRotator` (.roll (.rotation (`self.GetTransform`))) (.pitch (.rotation (`self.GetTransform`))) (+ (.yaw (.rotation (`self.GetTransform`))) (* (`GameplayStatics.GetWorldDeltaSeconds`) (`self.YawPerFrame`)))) (.scale _resttransform))))

(fn `UserConstructionScript`)